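; Doors500x is a sliding double door that opens when the player's MyCharacter enters its Activator trigger and closes when it leaves.
; Overlap events play a futuristic door sound and run the DoorsOpen timeline forward or in reverse.
; The timeline adds offsets, rotated by each door's world rotation, to start locations cached in the construction script, so each panel slides relative to its own orientation.
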(event `self.Activator.OnComponentBeginOverlap`
  (params (OtherActor :type "Actor Object Reference") (OtherComp :type "PrimitiveComponent Object Reference") (OtherBodyIndex :type Integer) (bFromSweep :type Boolean) (SweepResult :type "HitResult Structure (by ref)"))
  (bind _door2 (`self.Door2`))
  (bind _door1 (`self.Door1`))
  (cast `/Game/Blueprints/MyCharacter` OtherActor)
  (`GameplayStatics.PlaySound2D` "/Game/Sounds/Futuristic_door.Futuristic_door")
  (bind (_direction _door1open _door2open) (`Timeline|DoorsOpen` :!label _label)
    (:`Update`
      (`SceneComponent.K2_SetWorldLocation` _door1 (+ (`KismetMathLibrary.GreaterGreater_VectorRotator` _door1open (`SceneComponent.K2_GetComponentRotation` _door1)) (`self.Door1Start`)) false false)
      (`SceneComponent.K2_SetWorldLocation` _door2 (+ (`KismetMathLibrary.GreaterGreater_VectorRotator` _door2open (`SceneComponent.K2_GetComponentRotation` _door2)) (`self.Door2Start`)) false false))))

(event `self.Activator.OnComponentEndOverlap`
  (params (OtherActor :type "Actor Object Reference") (OtherComp :type "PrimitiveComponent Object Reference") (OtherBodyIndex :type Integer))
  (cast `/Game/Blueprints/MyCharacter` OtherActor)
  (`GameplayStatics.PlaySound2D` "/Game/Sounds/Futuristic_door.Futuristic_door")
  (goto _label :!via `Reverse`))

(fn `UserConstructionScript`
  (set `self.Door1Start` (`SceneComponent.K2_GetComponentLocation` (`self.Door1`)))
  (set `self.Door2Start` (`SceneComponent.K2_GetComponentLocation` (`self.Door2`))))