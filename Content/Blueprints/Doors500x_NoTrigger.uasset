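; Sliding double-door Blueprint that opens and closes through its OpenDoor and CloseDoor events, with no trigger logic of its own.
; The construction script caches both panels' world start locations.
; Each event plays a futuristic door sound and drives the DoorsOpen timeline forward or in reverse.
; Timeline offsets are rotated by each panel's world rotation and added to its start location, so movement follows the door's orientation.
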(event `Open Door`
  (bind _door2 (`self.Door2`))
  (bind _door1 (`self.Door1`))
  (`GameplayStatics.PlaySound2D` "/Game/Sounds/Futuristic_door.Futuristic_door")
  (bind (_direction _door1open _door2open) (`Timeline|DoorsOpen` :!label _label)
    (:`Update`
      (`SceneComponent.K2_SetWorldLocation` _door1 (+ (`KismetMathLibrary.GreaterGreater_VectorRotator` _door1open (`SceneComponent.K2_GetComponentRotation` _door1)) (`self.Door1Start`)) false false)
      (`SceneComponent.K2_SetWorldLocation` _door2 (+ (`KismetMathLibrary.GreaterGreater_VectorRotator` _door2open (`SceneComponent.K2_GetComponentRotation` _door2)) (`self.Door2Start`)) false false))))

(event `Close Door`
  (`GameplayStatics.PlaySound2D` "/Game/Sounds/Futuristic_door.Futuristic_door")
  (goto _label :!via `Reverse`))

(fn `UserConstructionScript`
  (set `self.Door1Start` (`SceneComponent.K2_GetComponentLocation` (`self.Door1`)))
  (set `self.Door2Start` (`SceneComponent.K2_GetComponentLocation` (`self.Door2`))))