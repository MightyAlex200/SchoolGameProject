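; Cube actor that moves under its own switchable vertical gravity and restarts the level when it drops to world height zero or below.
; Each tick it applies CubeGravity as a force to the Cube component while that simulates physics.
; Turnupsidedown reverses that force between strong upward and downward pull, and BeginPlay sets the actor's rotation to a half turn.
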(event `self.ReceiveTick`
  (params (DeltaSeconds :type "Float (single-precision)"))
  (bind (_returnvalue_x _returnvalue_y _returnvalue_z) (`KismetMathLibrary.BreakVector` (`self.K2_GetActorLocation`)))
  (if (<= _returnvalue_z 0.0)
    (`KismetSystemLibrary.ExecuteConsoleCommand` "restartlevel")
    (elif (`SceneComponent.IsSimulatingPhysics` (`self.Cube`) "None")
      (`PrimitiveComponent.AddForce` (`self.Cube`) (`self.CubeGravity`) "None" false))))

(event `Turn upsidedown`
  (bind (_cubegravity_x _cubegravity_y _cubegravity_z) (`KismetMathLibrary.BreakVector` (`self.CubeGravity`)))
  (if (< _cubegravity_z 0.0)
    (set `self.CubeGravity` (0.0 0.0 150000.0))
    (else
      (set `self.CubeGravity` (0.0 0.0 -150000.0)))))

(event `self.ReceiveBeginPlay`
  (`self.SetActorRotation` (struct :`Roll` 180.0)))

(fn `UserConstructionScript`)