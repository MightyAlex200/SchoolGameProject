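; SpinningCube is an actor that bobs vertically and reacts to how close player 0's character is.
; Each Tick accumulates time and interpolates the location toward a sine-based Z offset from its current position.
; The same Tick derives a linear falloff from player distance, driving both uniform scale and PointLight intensity.
; Below the falloff threshold the actor stays at minimum scale and the light turns off.
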(event `self.ReceiveTick`
  (params (DeltaSeconds :type "Float (single-precision)"))
  (bind _returnvalue (`self.K2_GetActorLocation`))
  (bind _pointlight (`self.PointLight`))
  (bind _returnvalue_2 (- 1.0 (* (`self.GetDistanceTo` (`GameplayStatics.GetPlayerCharacter` 0)) 0.001)))
  ;[1 1 1] Move it up and down (this is really complicated for some reason lol)
  (set `self.Seconds` (+ (`self.Seconds`) DeltaSeconds))
  (`self.K2_SetActorLocation` (`KismetMathLibrary.VInterpTo` _returnvalue (+ _returnvalue (`KismetMathLibrary.MakeVector` 0.0 0.0 (* (`KismetMathLibrary.Sin` (`self.Seconds`)) 100.0))) DeltaSeconds 1.0))
  ;[1 1 1] Change Size, also realllly complicated xdddddddd
  (if (<= _returnvalue_2 0.1)
    (`self.SetActorScale3D` (0.1 0.1 0.1))
    (`LightComponent.SetIntensity` _pointlight 0.0)
    (else
      (`self.SetActorScale3D` (`KismetMathLibrary.MakeVector` _returnvalue_2 _returnvalue_2 _returnvalue_2))
      (`LightComponent.SetIntensity` _pointlight (* _returnvalue_2 50000.0)))))

(fn `UserConstructionScript`)